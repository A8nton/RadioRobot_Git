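; BP_SimpleEnemy is an enemy that teleports between linked nodes on a looping timer.
; Each tick picks a random next point from its current node and moves only if that point is unoccupied and a random roll passes the manager's Agression value.
; A move swaps the nodes' Occupied flags and re-keys the enemy in BP_EnemyMenager's EnemyList by its new node.
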(event Custom|Move
  (bind _output_get (Variables|Default|SetNextPosition (.OutItem (Utilities|Array|Random (Variables|/Game/Blueprints/Enemy/BP_EnemyPoint.BP_EnemyPoint_C|GetNextPoints (Variables|Default|GetCurrentNode))))))
  (if (not (<= (Utilities|Array|Length (Variables|/Game/Blueprints/Enemy/BP_EnemyPoint.BP_EnemyPoint_C|GetNextPoints (Variables|Default|GetCurrentNode))) 0))
    (if (not (Variables|/Game/Blueprints/Enemy/BP_EnemyPoint.BP_EnemyPoint_C|GetOccupied _output_get))
      (if (<= (Math|Random|RandomFloatinRange 1.0 2e+01) (Variables|/Game/Blueprints/Enemy/BP_EnemyMenager.BP_EnemyMenager_C|GetAgression (Variables|Default|GetEnemyMenager)))
        (Utilities|Map|Remove (Variables|/Game/Blueprints/Enemy/BP_EnemyMenager.BP_EnemyMenager_C|GetEnemyList (Variables|Default|GetEnemyMenager)) (Variables|Default|GetCurrentNode))
        (Variables|/Game/Blueprints/Enemy/BP_EnemyPoint.BP_EnemyPoint_C|SetOccupied (Variables|Default|GetCurrentNode) false)
        (bind _output_get_2 (Variables|Default|SetCurrentNode (Variables|Default|GetNextPosition)))
        (Variables|/Game/Blueprints/Enemy/BP_EnemyPoint.BP_EnemyPoint_C|SetOccupied _output_get_2 true)
        (Utilities|Map|Add (Variables|/Game/Blueprints/Enemy/BP_EnemyMenager.BP_EnemyMenager_C|GetEnemyList (Variables|Default|GetEnemyMenager)) _output_get_2 self)
        (Transformation|SetActorTransform (Math|Transform|MakeTransform (Transformation|GetActorLocation (Variables|Default|GetNextPosition)) "0, 0, 0" "1.000000,1.000000,1.000000") false true)))))

(event EventBeginPlay
  (Utilities|FlowControl|Sequence
    (:then_0
      (bind _returnvalue (Actor|GetActorOfClass "/Game/Blueprints/Enemy/BP_EnemyMenager.BP_EnemyMenager_C"))
      (Variables|Default|SetEnemyMenager _returnvalue)
      (Variables|/Game/Blueprints/Enemy/BP_EnemyPoint.BP_EnemyPoint_C|SetOccupied (Variables|Default|GetCurrentNode) true))
    (:then_1
      (Utilities|Time|SetTimerbyEvent (delegate Custom|Move) (Variables|Default|GetMoveOpportunity) true))))

(event EventDestroyed)

(fn ConstructionScript)