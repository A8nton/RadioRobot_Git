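; BP_Turret is a turret that, when activated, destroys enemies registered at the points in its NextPoints list.
; It gets the BP_EnemyMenager actor on BeginPlay and looks up each point in that manager's EnemyList map.
; ActivateTurret pulses the Shoot flag through a short delay, while a second sequence branch immediately destroys matched enemies, frees their points and removes the map entries.
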(event Custom|ActivateTurret
  (bind _enemymenager (Variables|Default|GetEnemyMenager))
  (bind _enemylist (Variables|/Game/Blueprints/Enemy/BP_EnemyMenager.BP_EnemyMenager_C|GetEnemyList _enemymenager))
  (Utilities|FlowControl|Sequence
    (:then_0
      (Variables|Default|SetShoot true)
      (Utilities|FlowControl|Delay 0.2)
      (Variables|Default|SetShoot false))
    (:then_1
      (for _array_element (Variables|Default|GetNextPoints)
        (if (Utilities|Map|Contains _enemylist _array_element)
          (Actor|DestroyActor (.Value (Utilities|Map|Find (Variables|/Game/Blueprints/Enemy/BP_EnemyMenager.BP_EnemyMenager_C|GetEnemyList (Variables|Default|GetEnemyMenager)) _array_element)))
          (Variables|/Game/Blueprints/Enemy/BP_EnemyPoint.BP_EnemyPoint_C|SetOccupied _array_element false)
          (Utilities|Map|Remove _enemylist _array_element))))))

(event EventBeginPlay
  (bind _returnvalue (Actor|GetActorOfClass "/Game/Blueprints/Enemy/BP_EnemyMenager.BP_EnemyMenager_C"))
  (Variables|Default|SetEnemyMenager _returnvalue))

(fn ConstructionScript
  (|CallParentFunction))