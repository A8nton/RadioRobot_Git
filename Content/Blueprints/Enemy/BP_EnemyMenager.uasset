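; BP_EnemyMenager periodically spawns simple enemies at designated start points in the level.
; On BeginPlay it gathers all BP_EnemyPoint actors, records the indices of those flagged StartPosition, and starts a looping SpawnOpportunity timer.
; Each tick of that timer picks a random start point and, if unoccupied, rolls against Agression to spawn a BP_SimpleEnemy there, passing the point as its CurrentNode.
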(event Custom|SpawnEnemy
  (bind _output_get (Variables|Default|SetChosenNode (Utilities|Array|Get(acopy) (Variables|Default|GetEnemyPoints) (.OutItem (Utilities|Array|Random (Variables|Default|GetStartPosition))))))
  (if (not (Variables|/Game/Blueprints/Enemy/BP_EnemyPoint.BP_EnemyPoint_C|GetOccupied _output_get))
    (if (<= (Math|Random|RandomFloatinRange 1.0 2e+01) (Variables|Default|GetAgression))
      (Game|SpawnActorfromClass "/Game/Blueprints/Enemy/BP_SimpleEnemy.BP_SimpleEnemy_C" (Transformation|GetActorTransform (Variables|Default|GetChosenNode)) "Undefined" "MultiplyWithRoot" 0 (Variables|Default|GetChosenNode) 0))))

(event EventBeginPlay
  (Utilities|FlowControl|Sequence
    (:then_0
      (bind _outactors (Actor|GetAllActorsOfClass "/Game/Blueprints/Enemy/BP_EnemyPoint.BP_EnemyPoint_C"))
      (bind _output_get (Variables|Default|SetEnemyPoints _outactors))
      (for (_array_element _array_index) _output_get
        (if (Variables|/Game/Blueprints/Enemy/BP_EnemyPoint.BP_EnemyPoint_C|GetStartPosition _array_element)
          (Utilities|Array|Add (Variables|Default|GetStartPosition) _array_index))))
    (:then_1
      (Utilities|Time|SetTimerbyEvent (delegate Custom|SpawnEnemy) (Variables|Default|GetSpawnOpportunity) true))))

(fn ConstructionScript)