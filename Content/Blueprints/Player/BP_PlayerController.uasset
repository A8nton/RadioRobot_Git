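; Player controller Blueprint that can keep the mouse cursor locked to the center of the viewport.
; Every Tick calls the CenterMouse event, which checks the IsCenterMouse flag.
; When the flag is set, it moves player 0's cursor to half the viewport size, truncated to integer pixels.
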(event Custom|CenterMouse
  (bind _returnvalue (Viewport|GetViewportSize))
  ;[0.15 0.15 0.15 0.5] Mouse Centering
  (if (Variables|Default|GetIsCenterMouse)
    (Class|PlayerController|SetMouseLocation (Game|GetPlayerController 0) (Math|Float|Truncate (/ (.x _returnvalue) 2.0)) (Math|Float|Truncate (/ (.y _returnvalue) 2.0)))))

(event EventBeginPlay)

(event EventTick
  (params (DeltaSeconds :type Float%20%28single-precision%29))
  (CallFunction|CenterMouse))

(fn ConstructionScript)