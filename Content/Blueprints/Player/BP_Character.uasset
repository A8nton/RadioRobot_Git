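; BP_Character is the first-person player character, with Enhanced Input walk and look, CanRun-gated sprint and footstep audio.
; While IsPlayer is set, Tick runs an interaction line trace that highlights the hit component through custom depth.
; Clicking a highlighted actor clears IsPlayer and possesses BP_Robot, while Esc is a test shortcut for that possession.
; Jump, camera bobbing and pause-menu logic are present but disconnected.
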(event Custom|Begining)

(event Custom|Bobbing
  (bind _returnvalue (Transformation|GetVelocity))
  (bind _returnvalue_2 (Game|GetPlayerController 0))
  (bind _returnvalue_3 (Math|Vector|VectorLength _returnvalue))
  ;[0.15 0.15 0.15 0.5] CameraBobbing
  (if (> _returnvalue_3 0.0)
    (if (< _returnvalue_3 4e+02)
      (Game|Feedback|ClientStartCameraShake _returnvalue_2 "/Game/Blueprints/Player/Bobbing/Camera_Walk.Camera_Walk_C" 1.0 "CameraLocal" "0, 0, 0")
      (else
        (Game|Feedback|ClientStartCameraShake _returnvalue_2 "/Game/Blueprints/Player/Bobbing/Camera_Sprint.Camera_Sprint_C" 1.0 "CameraLocal" "0, 0, 0")))
    (else
      (Game|Feedback|ClientStartCameraShake _returnvalue_2 "/Game/Blueprints/Player/Bobbing/Camera_Idle.Camera_Idle_C" 1.0 "CameraLocal" "0, 0, 0"))))

(event Custom|Sound_Walk
  ;[0.15 0.15 0.15 0.5] WalkSounds
  (Utilities|FlowControl|Sequence
    (:then_0
      (if (> (Math|Vector|VectorLength (Transformation|GetVelocity)) 3e+02)
        (Utilities|FlowControl|Delay 0.4)
        (if (AI|Components|NavMovement|IsMovingonGround (Variables|Character|GetCharacterMovement))
          (Audio|Components|Audio|Play (Variables|Default|Getwalk) 0.0))))
    (:then_1
      (if (not (AI|Components|NavMovement|IsFalling (Variables|Character|GetCharacterMovement)))
        (if (not (Variables|Is|GetisLanded))
          (Variables|Is|SetisLanded true)
          (Audio|Components|Audio|Play (Variables|Default|Getwalk) 0.0))))))

(event Custom|Widgets)

(event Custom|Raycasting
  (bind (_start _end) (|GetStart/EndPos_3))
  ;[0.15 0.15 0.15 0.5] Interaction Raycast
  (bind (_outhit _returnvalue) (Collision|LineTraceByChannel _start _end "TraceTypeQuery1" false 0 "None"))
  (if _returnvalue
    (Utilities|IsValid (Variables|Default|GetLastHitActor)
      (:Is%20Valid
        (if (not (== (.HitActor (Collision|BreakHitResult _outhit)) (Variables|Default|GetLastHitActor)))
          (CallFunction|Highlight false)
          (switch name (Utilities|Array|Get(acopy) (Variables|/Script/Engine.Actor|GetTags (.HitActor (Collision|BreakHitResult _outhit)))) :!label _label
            (:interact
              (Variables|Default|SetLastHitActor (.HitActor (Collision|BreakHitResult _outhit)))
              (Variables|Default|SetLastHitComponent (.HitComponent (Collision|BreakHitResult _outhit)))
              (CallFunction|Highlight true)))))
      (:Is%20Not%20Valid
        (goto _label)))
    (else
      (Utilities|IsValid (Variables|Default|GetLastHitActor)
        (:Is%20Valid
          (CallFunction|Highlight false))))))

(event Custom|StopSprint
  ;[1 1 1] Character
  ;;[1 1 1] Sprint | Disabled
  (Variables|/Script/Engine.CharacterMovementComponent|SetMaxWalkSpeed (Variables|Character|GetCharacterMovement) 4e+02)
  (Variables|is|SetisShift false)
  (Audio|Components|Audio|SetSound (Variables|Default|Getwalk) "/Game/SFX/Player/Cue_Walk_Better.Cue_Walk_Better"))

(event Input|EnhancedActionEvents|EnhancedInputActionEsc
  (params (ActionValue :type Boolean) (ElapsedSeconds :type Float%20%28double-precision%29) (TriggeredSeconds :type Float%20%28double-precision%29) (InputAction :type Input%20Action%20Object%20Reference :default "/Game/Inputs/Movement/Esc.Esc"))
  ;[0.15 0.15 0.15 0.5] Testing Robot Possession
  (:Started
    (bind _returnvalue (Actor|GetActorOfClass "/Game/Blueprints/Robot/BP_Robot.BP_Robot_C"))
    (Pawn|Possess (Game|GetPlayerController 0) _returnvalue)))

(event Input|EnhancedActionEvents|EnhancedInputActionLook
  (params (ActionValue :type Vector%202D%20Structure) (ElapsedSeconds :type Float%20%28double-precision%29) (TriggeredSeconds :type Float%20%28double-precision%29) (InputAction :type Input%20Action%20Object%20Reference :default "/Game/Inputs/Movement/Look.Look"))
  (bind _mousesensivity (Variables|Movement|GetmouseSensivity))
  ;[1 1 1] Character
  ;;[1 1 1] Camera
  (if true
    (Pawn|Input|AddControllerYawInput (* (.x ActionValue) _mousesensivity))
    (Pawn|Input|AddControllerPitchInput (* (.y ActionValue) _mousesensivity))))

(event Input|EnhancedActionEvents|EnhancedInputActionJump
  (params (ActionValue :type Boolean) (ElapsedSeconds :type Float%20%28double-precision%29) (TriggeredSeconds :type Float%20%28double-precision%29) (InputAction :type Input%20Action%20Object%20Reference :default "/Game/Inputs/Movement/Jump.Jump"))
  ;[1 1 1] Character
  ;;[0.15 0.15 0.15 0.5] Jump | Disabled
)

(event Input|EnhancedActionEvents|EnhancedInputActionLMB
  (params (ActionValue :type Boolean) (ElapsedSeconds :type Float%20%28double-precision%29) (TriggeredSeconds :type Float%20%28double-precision%29) (InputAction :type Input%20Action%20Object%20Reference :default "/Game/Inputs/Movement/LMB.LMB"))
  (bind _lasthitactor (Variables|Default|GetLastHitActor))
  ;[0.15 0.15 0.15 0.5] Interacting on Click
  (:Started
    (Utilities|IsValid _lasthitactor
      (:Is%20Valid
        (switch name (Utilities|Array|Get(acopy) (Variables|/Script/Engine.Actor|GetTags _lasthitactor) 1)
          (:monitor
            (Variables|Default|SetisPlayer false)
            (CallFunction|Highlight false)
            (bind _returnvalue (Actor|GetActorOfClass "/Game/Blueprints/Robot/BP_Robot.BP_Robot_C"))
            (Default|Possess _returnvalue)
            (Pawn|Possess (Game|GetPlayerController 0) _returnvalue)))))))

(event Input|EnhancedActionEvents|EnhancedInputActionWalk
  (params (ActionValue :type Vector%202D%20Structure) (ElapsedSeconds :type Float%20%28double-precision%29) (TriggeredSeconds :type Float%20%28double-precision%29) (InputAction :type Input%20Action%20Object%20Reference :default "/Game/Inputs/Movement/Walk.Walk"))
  (bind _returnvalue (Pawn|GetControlRotation :!class /Script/Engine.Pawn))
  (bind _walk (Variables|Default|Getwalk))
  ;[1 1 1] Character
  ;;[1 1 1] Movement
  (:Triggered
    (Pawn|Input|AddMovementInput (Math|Vector|GetRightVector (Math|Rotator|MakeRotator (.roll _returnvalue) 0.0 (.yaw _returnvalue))) (.x ActionValue) false)
    (Pawn|Input|AddMovementInput (Math|Vector|GetForwardVector (Math|Rotator|MakeRotator 0.0 0.0 (.yaw (Pawn|GetControlRotation :!class /Script/Engine.Pawn)))) (.y ActionValue) false))
  (:Started
    (Variables|Movement|SetisWalk true)
    (Variables|/Script/Engine.AudioComponent|SetVolumeMultiplier _walk 1.0)
    (if (not (Audio|Components|Audio|IsPlaying _walk))
      (if (not (Variables|is|GetisShift))
        (if (AI|Components|NavMovement|IsMovingonGround (Variables|Character|GetCharacterMovement))
          (Audio|Components|Audio|Play _walk 0.0)))))
  (:Completed
    (Variables|Movement|SetisWalk false)
    (Variables|/Script/Engine.AudioComponent|SetVolumeMultiplier _walk 0.0)))

(event Input|EnhancedActionEvents|EnhancedInputActionSprint
  (params (ActionValue :type Boolean) (ElapsedSeconds :type Float%20%28double-precision%29) (TriggeredSeconds :type Float%20%28double-precision%29) (InputAction :type Input%20Action%20Object%20Reference :default "/Game/Inputs/Movement/Sprint.Sprint"))
  (bind _charactermovement (Variables|Character|GetCharacterMovement))
  (bind _walk (Variables|Default|Getwalk))
  ;[1 1 1] Character
  ;;[1 1 1] Sprint | Disabled
  (:Started
    (if (Variables|Movement|GetcanRun)
      (Variables|/Script/Engine.CharacterMovementComponent|SetMaxWalkSpeed _charactermovement 6e+02)
      (Variables|is|SetisShift true)
      (Audio|Components|Audio|SetSound _walk "/Game/SFX/Cue_Walk.Cue_Walk")))
  (:Completed
    (Variables|/Script/Engine.CharacterMovementComponent|SetMaxWalkSpeed _charactermovement 4e+02)
    (Variables|is|SetisShift false)
    (Audio|Components|Audio|SetSound _walk "/Game/SFX/Player/Cue_Walk_Better.Cue_Walk_Better")))

(event EventTick
  (params (DeltaSeconds :type Float%20%28single-precision%29))
  (if (Variables|Default|GetisPlayer)
    (Variables|Default|SetDelta%20Seconds DeltaSeconds)
    (Utilities|FlowControl|Sequence
      (:then_0
        (CallFunction|Raycasting))
      (:then_1
        (CallFunction|SoundWalk)))))

(event EventBeginPlay
  ;[1 1 1] Character
  ;;[1 1 1] Initial
  (Utilities|FlowControl|Sequence
    (:then_0
      (bind _asplayer_controller (Utilities|Casting|CastToPlayerController (Pawn|GetController)))
      (Utilities|IsValid (PlayerController|LocalPlayerSubsystems|GetEnhancedInputLocalPlayerSubsystem _asplayer_controller)
        (:Is%20Valid
          (Input|AddMappingContext (PlayerController|LocalPlayerSubsystems|GetEnhancedInputLocalPlayerSubsystem _asplayer_controller) "/Game/Inputs/BasicInput.BasicInput" 0 "(bIgnoreAllPressedKeysUntilRelease=True,bForceImmediately=False,bNotifyUserSettings=False)"))))
    (:then_1
      (CallFunction|Begining)
      (CallFunction|Widgets))))

(fn ConstructionScript)

(fn Highlight
  (params (isOn :type Boolean))
  (Rendering|SetRenderCustomDepth (Variables|Default|GetLastHitComponent) isOn)
  (if (not isOn)
    (Variables|Default|SetLastHitActor 0)
    (Variables|Default|SetLastHitComponent 0)))