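; BP_Node is one grid cell of the generated cave, trimming its own walls where it borders other nodes.
; On BeginPlay it binds to the NodeManager's update-walls event, which triggers UpdateWalls.
; UpdateWalls looks up the four X/Y neighbors of GridPos in the manager's ListOfNodes.
; Indexes of occupied sides are collected and removed together from the instanced CaveWall, opening passages between adjacent nodes.
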(event Custom|StartUpdateWalls
  (CallFunction|UpdateWalls))

(event EventBeginPlay
  (EventDispatchers|BindEventtoUpdateWallsEvent (Variables|Default|GetNodeManager) (delegate Custom|StartUpdateWalls)))

(fn ConstructionScript)

(fn UpdateWalls
  (bind _gridpos (Variables|Default|GetGridPos))
  (bind _gridpos_2 (Variables|Default|GetGridPos))
  (bind _gridpos_3 (Variables|Default|GetGridPos))
  (bind _gridpos_4 (Variables|Default|GetGridPos))
  (for _index (range 0 3)
    (switch int _index
      (:0
        (if (.ReturnValue (Utilities|Map|Find (Variables|/Game/Blueprints/Cave/CaveGeneration/BP_CaveGeneration.BP_CaveGeneration_C|GetListOfNodes (Variables|Default|GetNodeManager)) (Math|Vector|MakeVector (.x _gridpos_4) (+ (.y _gridpos_4) 1.0) (.z _gridpos_4))))
          (Utilities|Array|Add (LocalVariables|GetRemoveIndexes) _index :!label _label)))
      (:1
        (if (.ReturnValue (Utilities|Map|Find (Variables|/Game/Blueprints/Cave/CaveGeneration/BP_CaveGeneration.BP_CaveGeneration_C|GetListOfNodes (Variables|Default|GetNodeManager)) (Math|Vector|MakeVector (+ (.x _gridpos) 1.0) (.y _gridpos) (.z _gridpos))))
          (goto _label)))
      (:2
        (if (.ReturnValue (Utilities|Map|Find (Variables|/Game/Blueprints/Cave/CaveGeneration/BP_CaveGeneration.BP_CaveGeneration_C|GetListOfNodes (Variables|Default|GetNodeManager)) (Math|Vector|MakeVector (.x _gridpos_3) (+ (.y _gridpos_3) -1.0) (.z _gridpos_3))))
          (goto _label)))
      (:3
        (if (.ReturnValue (Utilities|Map|Find (Variables|/Game/Blueprints/Cave/CaveGeneration/BP_CaveGeneration.BP_CaveGeneration_C|GetListOfNodes (Variables|Default|GetNodeManager)) (Math|Vector|MakeVector (+ (.x _gridpos_2) -1.0) (.y _gridpos_2) (.z _gridpos_2))))
          (goto _label)))))
  (Class|InstancedStaticMeshComponent|RemoveInstances (Variables|Default|GetCave_Wall) (LocalVariables|GetRemoveIndexes)))