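; BP_CaveGeneration builds a cave layout at BeginPlay by growing random "snakes" of node actors on a grid, instantly or step by step with delays.
; GenerateNode extends a snake into free cells with under three neighbors, ending it early when crowded.
; Snake ends become branch points until their four-way neighbors fill up.
; A temporary node reserves a wall spot for a button, then is removed before walls update.
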(event Custom|TestSpawnNode
  (params (GridPos :type Vector))
  (bind _self self)
  (bind _returnvalue (Transformation|GetActorTransform _self))
  (bind _returnvalue_2 (Game|SpawnActorfromClass (Variables|Default|GetBP_NodeClass) (Math|Transform|MakeTransform (+ (* GridPos "200.000000,200.000000,0.000000") (.location _returnvalue)) (.rotation _returnvalue) (.scale _returnvalue)) "Undefined" "MultiplyWithRoot" 0 GridPos _self 0))
  (Utilities|Map|Add (Variables|Default|GetListOfNodes) (Variables|/Game/Blueprints/Cave/CaveGeneration/BP_Node.BP_Node_C|GetGridPos _returnvalue_2) _returnvalue_2))

(event EventBeginPlay
  (bind _self self)
  (bind _listofnodes (Variables|Default|GetListOfNodes))
  (bind _listofnodes_2 (Variables|Default|GetListOfNodes))
  ;[0.15 0.15 0.15 0.5] Spawns first node
  (bind _returnvalue (Game|SpawnActorfromClass (Variables|Default|GetBP_NodeClass) (Transformation|GetActorTransform _self) "Undefined" "MultiplyWithRoot" 0 "0.000000,0.000000,0.000000" _self 0))
  (Utilities|Map|Add (Variables|Default|GetListOfNodes) (Variables|/Game/Blueprints/Cave/CaveGeneration/BP_Node.BP_Node_C|GetGridPos _returnvalue) _returnvalue)
  (Utilities|Map|Add (Variables|Default|GetListOfHeadNodes) (Variables|/Game/Blueprints/Cave/CaveGeneration/BP_Node.BP_Node_C|GetGridPos _returnvalue) _returnvalue)
  (Rendering|SetVisibility (Variables|/Game/Blueprints/Cave/CaveGeneration/BP_Node.BP_Node_C|GetCave_Ceiling _returnvalue) false false)
  (CallFunction|TestSpawnNode "0.000000,-1.000000,0.000000")
  (if (Variables|Default|GetIsInstantGeneration)
    (for _index (range 1 (Variables|Default|GetAmountOfSnakes))
      (Utilities|FlowControl|ForLoopwithBreak 1 (Variables|Default|GetSnakeLength) :!label _label
        (:LoopBody
          (bind (_secsesfulgenerationofnode _newnode _snakeendsearly) (CallFunction|GenerateNode (Variables|Default|GetLastNodeSpawned)))
          (Variables|Default|SetLastNodeSpawned _newnode)
          (if _snakeendsearly
            (goto _label Break)))
        (:Completed
          (bind _lastnodespawned (Variables|Default|GetLastNodeSpawned)
            (:then
              (Utilities|Map|Add (Variables|Default|GetListOfHeadNodes) (Variables|/Game/Blueprints/Cave/CaveGeneration/BP_Node.BP_Node_C|GetGridPos _lastnodespawned) _lastnodespawned))
            (:else
              _))
          (Variables|Default|SetLastNodeSpawned 0)
          (bind (_keypin _valuepin) (Utilities|Map|ForEachLoop(Map) (Variables|Default|GetListOfHeadNodes))
            (:then
              (bind _amountofneighbors (CallFunction|CheckNeighbors _valuepin false "0, 0, 0"))
              (if (>= _amountofneighbors 3)
                (Utilities|Map|Remove (Variables|Default|GetListOfHeadNodes) _keypin)))))))
    ;[0.15 0.15 0.15 0.5] Always have a wall to spawn button on
    (Actor|DestroyActor (.Value (Utilities|Map|Find _listofnodes "0.000000,-1.000000,0.000000")))
    (Utilities|Map|Remove _listofnodes "0.000000,-1.000000,0.000000")
    (Default|CallUpdateWallsEvent)
    (else
      (Utilities|FlowControl|Delay 0.7 :!label _label_2)
      (if (>= (Variables|Default|GetCurSnakeLength) (Variables|Default|GetSnakeLength)) :!label _label_3
        _
        (else
          (Utilities|FlowControl|Delay 0.2)
          (bind (_secsesfulgenerationofnode_2 _newnode_2 _snakeendsearly_2) (CallFunction|GenerateNode (Variables|Default|GetLastNodeSpawned)))
          (Variables|Default|SetLastNodeSpawned _newnode_2)
          (Math|Integer|IncrementInt (Variables|Default|GetCurSnakeLength)
            (:%20%20
              (if _snakeendsearly_2
                _
                (else
                  (goto _label_3)))))))
      (bind _lastnodespawned_2 (Variables|Default|GetLastNodeSpawned)
        (:then
          (Utilities|Map|Add (Variables|Default|GetListOfHeadNodes) (Variables|/Game/Blueprints/Cave/CaveGeneration/BP_Node.BP_Node_C|GetGridPos _lastnodespawned_2) _lastnodespawned_2))
        (:else
          _))
      (Math|Integer|IncrementInt (Variables|Default|GetCurAmountOfSnakes)
        (:%20%20
          (Variables|Default|SetCurSnakeLength 0)
          (Variables|Default|SetLastNodeSpawned 0)
          (bind (_keypin_2 _valuepin_2) (Utilities|Map|ForEachLoop(Map) (Variables|Default|GetListOfHeadNodes))
            (:then
              (bind _amountofneighbors_2 (CallFunction|CheckNeighbors _valuepin_2 false "0, 0, 0"))
              (if (>= _amountofneighbors_2 3)
                (Utilities|Map|Remove (Variables|Default|GetListOfHeadNodes) _keypin_2)))
            (:CompletedPin
              (if (>= (Variables|Default|GetCurAmountOfSnakes) (Variables|Default|GetAmountOfSnakes))
                (Development|PrintString "Generation Ends")
                (Utilities|FlowControl|Delay 0.5)
                ;[0.15 0.15 0.15 0.5] Always have a wall to spawn button on
                (Actor|DestroyActor (.Value (Utilities|Map|Find _listofnodes_2 "0.000000,-1.000000,0.000000")))
                (Utilities|Map|Remove _listofnodes_2 "0.000000,-1.000000,0.000000")
                (Utilities|FlowControl|Delay 0.5)
                (Default|CallUpdateWallsEvent)
                (else
                  (goto _label_2))))))))))

(fn ConstructionScript)

(fn GenerateNode
  (params (ChoosenNode :type BP%20Node%20Object%20Reference))
  (bind _avaliabledirections (LocalVariables|GetAvaliableDIrections))
  (bind _choosennode (LocalVariables|GetChoosenNode)
    (:then
      (LocalVariables|SetNode _choosennode))
    (:else
      ;[0.15 0.15 0.15 0.5] Pick Random Node
      (bind _values (Utilities|Map|Values (Variables|Default|GetListOfHeadNodes)))
      (LocalVariables|SetNode (.OutItem (Utilities|Array|Random _values)))))
  (for _array_element (LocalVariables|GetDirections)
    (if (not (Utilities|Map|IsEmpty (Variables|Default|GetListOfHeadNodes)))
      (if (not (Utilities|Map|Contains (Variables|Default|GetListOfNodes) (+ (Variables|/Game/Blueprints/Cave/CaveGeneration/BP_Node.BP_Node_C|GetGridPos (LocalVariables|GetNode)) _array_element)))
        (Utilities|Array|Add (LocalVariables|GetAvaliableDIrections) _array_element))))
  (if (<= (Utilities|Array|Length (LocalVariables|GetAvaliableDIrections)) 0)
    (return false 0 false)
    (else
      (for _array_element_2 _avaliabledirections
        (bind _amountofneighbors (CallFunction|CheckNeighbors 0 true (+ _array_element_2 (Variables|/Game/Blueprints/Cave/CaveGeneration/BP_Node.BP_Node_C|GetGridPos (LocalVariables|GetNode)))))
        (if (>= _amountofneighbors 3)
          (Utilities|Array|RemoveItem _avaliabledirections _array_element_2)))
      (if (Utilities|Array|IsEmpty (LocalVariables|GetAvaliableDIrections))
        (return false 0 true)
        (else
          (LocalVariables|SetDirection (.OutItem (Utilities|Array|Random (LocalVariables|GetAvaliableDIrections))))
          ;[0.15 0.15 0.15 0.5] Spawns Node at location
          (bind _returnvalue (Game|SpawnActorfromClass (Variables|Default|GetBP_NodeClass) (Math|Transform|MakeTransform (+ (* (LocalVariables|GetDirection) (LocalVariables|GetDistanceBetweenNodes)) (.location (Transformation|GetActorTransform (LocalVariables|GetNode)))) (.rotation (Transformation|GetActorTransform (LocalVariables|GetNode))) (.scale (Transformation|GetActorTransform (LocalVariables|GetNode)))) "Undefined" "MultiplyWithRoot" 0 (+ (LocalVariables|GetDirection) (Variables|/Game/Blueprints/Cave/CaveGeneration/BP_Node.BP_Node_C|GetGridPos (LocalVariables|GetNode))) self 0))
          (Utilities|Map|Add (Variables|Default|GetListOfNodes) (Variables|/Game/Blueprints/Cave/CaveGeneration/BP_Node.BP_Node_C|GetGridPos _returnvalue) _returnvalue)
          (return true _returnvalue false))))))

(fn CheckNeighbors
  (params (Node :type BP%20Node%20Object%20Reference) (CheckAllNeighbors :type Boolean) (Location :type Vector))
  (bind _node (LocalVariables|GetNode)
    (:then
      (LocalVariables|SetLocToCheckAt (Variables|/Game/Blueprints/Cave/CaveGeneration/BP_Node.BP_Node_C|GetGridPos _node)))
    (:else
      (LocalVariables|SetLocToCheckAt Location)))
  (if CheckAllNeighbors
    (for _array_element (LocalVariables|GetDirections)
      (if (Utilities|Map|Contains (Variables|Default|GetListOfNodes) (+ (LocalVariables|GetLocToCheckAt) _array_element))
        (Math|Integer|IncrementInt (LocalVariables|GetResults))))
    (return (LocalVariables|GetResults) 8)
    (else
      (for _array_element_2 (LocalVariables|GetLimitedDirection)
        (if (Utilities|Map|Contains (Variables|Default|GetListOfNodes) (+ (LocalVariables|GetLocToCheckAt) _array_element_2))
          (Math|Integer|IncrementInt (LocalVariables|GetResults))))
      (return (LocalVariables|GetResults) 4))))