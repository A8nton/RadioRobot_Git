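; Depot basket that collects deposited money, displays it as gold bars and extracts it when full.
; On BeginPlay it recursively caches the Gold mesh instance transforms, then resets the instances to a zero transform.
; PlaceItems accumulates money and restores bars in four value tiers.
; The top tier triggers Extract, which launches BP_Depot_Base, waits, credits the total to BP_ValuesManager and empties the basket.
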(event Custom|GetInstanceTransform
  (bind _gold (Variables|Default|GetGold))
  ;[0.15 0.15 0.15 0.5] Method for remembering gold bar positions
  (if (<= (Variables|Default|GetTemp_InstanceIndex) (Components|InstancedStaticMesh|GetInstanceCount _gold))
    (Utilities|Array|Add (Variables|Default|GetGoldTransforms) (.OutInstanceTransform (Components|InstancedStaticMesh|GetInstanceTransform _gold (Variables|Default|GetTemp_InstanceIndex) false)))
    (Math|Integer|IncrementInt (Variables|Default|GetTemp_InstanceIndex)
      (:%20%20
        (CallFunction|GetInstanceTransform)))
    (else
      (Development|PrintString "Finalized Gold Transform")
      (CallFunction|ResetInstanceTransform))))

(event Custom|PlaceItems
  (params (Money :type Integer))
  ;[0.15 0.15 0.15 0.5] Fires when player interacts with it. Based on price of players inventory shows 4 different gold positions. inv < 5k = 5 gold | 5k < inv < 10k = 10 gold | 10k < inv < 15k = 15 gold | 15k < inv < 20k = 20 gold, after the 20 gold visible the extractor would automaticaly start extracting the gold to the surface. Also there is possibility to put inside more that 20k worth of gold so the depot is smart enough to accept it also, it won't delete the rest. After the extraction it adds the ammount of extracted money to the values manager to store.
  (bind _output_get (Variables|Default|SetCurrentMoney (+ Money (Variables|Default|GetCurrentMoney))))
  (if (Math|Integer|InRange(Integer) _output_get 100 5000)
    (Variables|Default|SetVisibleGold 4)
    (CallFunction|SetPosBasedonIndex (Variables|Default|GetVisibleGold) :!label _label)
    (if (== (Variables|Default|GetVisibleGold) 19)
      (CallFunction|Extract))
    (elif (Math|Integer|InRange(Integer) _output_get 5001 10000)
      (Variables|Default|SetVisibleGold 9)
      (goto _label)
      (elif (Math|Integer|InRange(Integer) _output_get 10001 15000)
        (Variables|Default|SetVisibleGold 14)
        (goto _label)
        (elif (Math|Integer|InRange(Integer) _output_get 15001 20000)
          (Variables|Default|SetVisibleGold 19)
          (goto _label)
          (elif (Math|Integer|InRange(Integer) _output_get 20001 40000)
            (Variables|Default|SetVisibleGold 19)
            (goto _label)
            (else
              (Development|PrintString (Utilities|String|Append "Player has $" (Utilities|String|ToString(Integer) Money))))))))))

(event Custom|Extract
  ;[0.15 0.15 0.15 0.5] Extraction sequence
  (Development|PrintString "Extracting gold")
  (bind _returnvalue (Actor|GetActorOfClass "/Game/Blueprints/Robot/BP_Depot_Base.BP_Depot_Base_C"))
  (Default|ExtractLaunch _returnvalue)
  (Utilities|FlowControl|Delay 2.0)
  (Default|AddMoney (Variables|Default|GetManager) (Variables|Default|GetCurrentMoney))
  (Development|PrintString "Extracted")
  (CallFunction|ResetInstanceTransform))

(event EventBeginPlay
  ;[0.15 0.15 0.15 0.5] Remembers position of each gold bar, gets values manager to pass money value to it after the extraction
  (CallFunction|GetInstanceTransform)
  (bind _returnvalue (Actor|GetActorOfClass "/Game/Blueprints/BP_ValuesManager.BP_ValuesManager_C"))
  (Variables|Default|SetManager _returnvalue))

(fn ConstructionScript)

(fn SetPosBasedonIndex
  (params (MaxIndex :type Integer))
  (for _index (range (LocalVariables|Getindex) MaxIndex)
    (Components|InstancedStaticMesh|UpdateInstanceTransform (Variables|Default|GetGold) _index (Utilities|Array|Get(acopy) (Variables|Default|GetGoldTransforms) _index) false false false)))

(fn ResetInstanceTransform
  (bind _gold (Variables|Default|GetGold))
  (for _index (range 0 (Components|InstancedStaticMesh|GetInstanceCount _gold))
    (Components|InstancedStaticMesh|UpdateInstanceTransform _gold _index (Variables|Default|GetZeroTransform) false false false)
    (Variables|Default|SetCurrentMoney 0)
    (Variables|Default|SetVisibleGold 0)))