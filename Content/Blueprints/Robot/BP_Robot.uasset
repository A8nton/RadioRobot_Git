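; Possessable first-person robot that collects priced loot, deposits it at a depot and presses extraction buttons.
; While possessed, Tick runs camera shakes, footsteps and a line trace that outlines targets via custom depth and shows gold prices on WB_Robot.
; E interacts by actor tag; loot price sets inventory weight, which slows walking and blocks sprint when overloaded.
; F toggles the flashlight; holding Q returns control to BP_Character.
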(event Custom|Begining
  (bind _returnvalue (Actor|GetActorOfClass "/Game/Blueprints/Player/BP_Character.BP_Character_C"))
  (Variables|Default|SetPlayerRef _returnvalue))

(event Custom|Bobbing
  (bind _returnvalue (Transformation|GetVelocity))
  (bind _returnvalue_2 (Game|GetPlayerController 0))
  (bind _returnvalue_3 (Math|Vector|VectorLength _returnvalue))
  ;[0.15 0.15 0.15 0.5] CameraBobbing
  (if (> _returnvalue_3 0.0)
    (if (< _returnvalue_3 4e+02)
      (Game|Feedback|ClientStartCameraShake _returnvalue_2 "/Game/Blueprints/Player/Bobbing/Camera_Walk.Camera_Walk_C" 1.0 "CameraLocal" "0, 0, 0")
      (else
        (Game|Feedback|ClientStartCameraShake _returnvalue_2 "/Game/Blueprints/Player/Bobbing/Camera_Sprint.Camera_Sprint_C" 1.0 "CameraLocal" "0, 0, 0")))
    (else
      (Game|Feedback|ClientStartCameraShake _returnvalue_2 "/Game/Blueprints/Player/Bobbing/Camera_Idle.Camera_Idle_C" 1.0 "CameraLocal" "0, 0, 0"))))

(event Custom|Sound_Walk
  (bind _returnvalue (Transformation|GetVelocity))
  (bind _returnvalue_2 (Math|Vector|VectorLength _returnvalue))
  ;[0.15 0.15 0.15 0.5] WalkSounds
  (Utilities|FlowControl|Sequence
    (:then_0
      (if (> _returnvalue_2 3e+02)
        (Utilities|FlowControl|Delay 0.4)
        (if (AI|Components|NavMovement|IsMovingonGround (Variables|Character|GetCharacterMovement)) :!label _label
          (Audio|Components|Audio|Play (Variables|Default|Getwalk) 0.0))
        (elif (> _returnvalue_2 2e+02)
          (if (Variables|Is|GetisOverflow)
            (Utilities|FlowControl|Delay 0.6)
            (goto _label)))))))

(event Custom|Widgets)

(event Custom|Possess
  ;[0.15 0.15 0.15 0.5] Robot Functionality
  (bind _returnvalue (UserInterface|CreateWidget "/Game/UI/Game/Robot/WB_Robot.WB_Robot_C"))
  (bind _output_get (Variables|Default|SetRobotWidget _returnvalue))
  (UserInterface|Viewport|AddtoViewport _output_get 0)
  (Variables|Is|SetisPossessed true))

(event Custom|UnPossess
  (bind _last_hit_actor (Variables|Default|GetLast%20Hit%20Actor))
  (bind _playerref (Variables|Default|GetPlayerRef))
  ;[0.15 0.15 0.15 0.5] Robot Functionality
  (Widget|RemovefromParent (Variables|Default|GetRobotWidget))
  (Variables|Is|SetisPossessed false)
  (Utilities|IsValid _last_hit_actor
    (:Is%20Valid
      (CallFunction|Highlight _last_hit_actor false (Variables|Default|GetLastHitComponent)))
    (:Is%20Not%20Valid
      _))
  (Pawn|Possess (Game|GetPlayerController 0) _playerref)
  (Variables|/Game/Blueprints/Player/BP_Character.BP_Character_C|SetisPlayer _playerref true))

(event Custom|Outline
  (bind (_start _end) (|GetStart/EndPos_3_2_2))
  ;[0.15 0.15 0.15 0.5] Permanent Raycast
  (bind (_outhit _returnvalue) (Collision|LineTraceByChannel _start _end "TraceTypeQuery1" false 0 "None"))
  (if _returnvalue
    (Utilities|IsValid (Variables|Default|GetLast%20Hit%20Actor)
      (:Is%20Valid
        (if (== (.HitActor (Collision|BreakHitResult _outhit)) (Variables|Default|GetLast%20Hit%20Actor))
          _
          (else
            (CallFunction|Highlight (Variables|Default|GetLast%20Hit%20Actor) false (Variables|Default|GetLastHitComponent)))))
      (:Is%20Not%20Valid
        _))
    (switch name (Utilities|Array|Get(acopy) (Variables|/Script/Engine.Actor|GetTags (.HitActor (Collision|BreakHitResult _outhit))))
      (:interact
        (bind _output_get (Variables|Default|SetLast%20Hit%20Actor (.HitActor (Collision|BreakHitResult _outhit))))
        (bind _output_get_2 (Variables|Default|SetLastHitComponent (.HitComponent (Collision|BreakHitResult _outhit))))
        (CallFunction|Highlight _output_get true _output_get_2)))
    (else
      (Utilities|IsValid (Variables|Default|GetLast%20Hit%20Actor)
        (:Is%20Valid
          (CallFunction|Highlight (Variables|Default|GetLast%20Hit%20Actor) false (Variables|Default|GetLastHitComponent)))))))

(event Custom|StopSprint
  ;[1 1 1] Character
  ;;[1 1 1] Sprint
  (Variables|/Script/Engine.CharacterMovementComponent|SetMaxWalkSpeed (Variables|Character|GetCharacterMovement) (Variables|Movement|GetMaxSpeedWalk))
  (Variables|is|SetisShift false)
  (Audio|Components|Audio|SetSound (Variables|Default|Getwalk) "/Game/SFX/Player/Cue_Walk_Better.Cue_Walk_Better"))

(event Input|EnhancedActionEvents|EnhancedInputActionEsc
  (params (ActionValue :type Boolean) (ElapsedSeconds :type Float%20%28double-precision%29) (TriggeredSeconds :type Float%20%28double-precision%29) (InputAction :type Input%20Action%20Object%20Reference :default "/Game/Inputs/Movement/Esc.Esc")))

(event Input|EnhancedActionEvents|EnhancedInputActionLook
  (params (ActionValue :type Vector%202D%20Structure) (ElapsedSeconds :type Float%20%28double-precision%29) (TriggeredSeconds :type Float%20%28double-precision%29) (InputAction :type Input%20Action%20Object%20Reference :default "/Game/Inputs/Movement/Look.Look"))
  (bind _mousesensivity (Variables|Movement|GetmouseSensivity))
  ;[1 1 1] Character
  ;;[1 1 1] Camera
  (if true
    (Pawn|Input|AddControllerYawInput (* (.x ActionValue) _mousesensivity))
    (Pawn|Input|AddControllerPitchInput (* (.y ActionValue) _mousesensivity))))

(event Input|EnhancedActionEvents|EnhancedInputActionJump
  (params (ActionValue :type Boolean) (ElapsedSeconds :type Float%20%28double-precision%29) (TriggeredSeconds :type Float%20%28double-precision%29) (InputAction :type Input%20Action%20Object%20Reference :default "/Game/Inputs/Movement/Jump.Jump"))
  ;[1 1 1] Character
  ;;[0.15 0.15 0.15 0.5] Jump | Turned off
)

(event Input|EnhancedActionEvents|EnhancedInputActionQ_Key
  (params (ActionValue :type Boolean) (ElapsedSeconds :type Float%20%28double-precision%29) (TriggeredSeconds :type Float%20%28double-precision%29) (InputAction :type Input%20Action%20Object%20Reference :default "/Game/Inputs/Movement/Q_Key.Q_Key"))
  ;[0.15 0.15 0.15 0.5] Robot Functionality
  (:Started
    (Variables|Default|SetisQ true)
    (Utilities|FlowControl|Delay 0.5)
    (if (Variables|Default|GetisQ)
      (CallFunction|UnPossess)))
  (:Completed
    (Variables|Default|SetisQ false)))

(event Input|EnhancedActionEvents|EnhancedInputActionF_Key
  (params (ActionValue :type Boolean) (ElapsedSeconds :type Float%20%28double-precision%29) (TriggeredSeconds :type Float%20%28double-precision%29) (InputAction :type Input%20Action%20Object%20Reference :default "/Game/Inputs/Movement/F_Key.F_Key"))
  (bind _spotlight (Variables|Default|GetSpotLight))
  ;[0.15 0.15 0.15 0.5] Robot Functionality
  (:Started
    (if (Variables|Is|GetisPossessed)
      (Utilities|FlowControl|FlipFlop
        (:A
          (Variables|Is|SetisFlashLight true)
          (Rendering|Components|Light|SetIntensity _spotlight 2e+01))
        (:B
          (Variables|Is|SetisFlashLight false)
          (Rendering|Components|Light|SetIntensity _spotlight 0.0))))))

(event Input|EnhancedActionEvents|EnhancedInputActionE_Key
  (params (ActionValue :type Boolean) (ElapsedSeconds :type Float%20%28double-precision%29) (TriggeredSeconds :type Float%20%28double-precision%29) (InputAction :type Input%20Action%20Object%20Reference :default "/Game/Inputs/Movement/E_Key.E_Key"))
  (bind _last_hit_actor (Variables|Default|GetLast%20Hit%20Actor))
  ;[0.15 0.15 0.15 0.5] Robot Interaction
  (:Started
    (if (Variables|Is|GetisPossessed)
      (Utilities|IsValid _last_hit_actor
        (:Is%20Valid
          (switch name (Utilities|Array|Get(acopy) (Variables|/Script/Engine.Actor|GetTags _last_hit_actor) 1)
            (:gold
              (bind _asbp_test_val_robot (Utilities|Casting|CastToBP_TestValRobot _last_hit_actor))
              (CallFunction|DetermineValue _asbp_test_val_robot))
            (:basket
              (bind _asbp_depot (Utilities|Casting|CastToBP_Depot _last_hit_actor))
              (Default|PlaceItems _asbp_depot (Variables|Inventory|GetInventoryPrice))
              (CallFunction|RemoveItemsfromInv))
            (:button
              (bind _asbp_button (Utilities|Casting|CastToBP_Button _last_hit_actor))
              (Default|LaunchExtract _asbp_button))))))))

(event Input|EnhancedActionEvents|EnhancedInputActionWalk
  (params (ActionValue :type Vector%202D%20Structure) (ElapsedSeconds :type Float%20%28double-precision%29) (TriggeredSeconds :type Float%20%28double-precision%29) (InputAction :type Input%20Action%20Object%20Reference :default "/Game/Inputs/Movement/Walk.Walk"))
  (bind _returnvalue (Pawn|GetControlRotation :!class /Script/Engine.Pawn))
  (bind _walk (Variables|Default|Getwalk))
  ;[1 1 1] Character
  ;;[1 1 1] Movement
  (:Triggered
    (Pawn|Input|AddMovementInput (Math|Vector|GetRightVector (Math|Rotator|MakeRotator (.roll _returnvalue) 0.0 (.yaw _returnvalue))) (.x ActionValue) false)
    (Pawn|Input|AddMovementInput (Math|Vector|GetForwardVector (Math|Rotator|MakeRotator 0.0 0.0 (.yaw (Pawn|GetControlRotation :!class /Script/Engine.Pawn)))) (.y ActionValue) false))
  (:Started
    (Variables|Movement|SetisWalk true)
    (Variables|/Script/Engine.AudioComponent|SetVolumeMultiplier _walk 1.0)
    (if (not (Audio|Components|Audio|IsPlaying _walk))
      (if (not (Variables|is|GetisShift))
        (if (AI|Components|NavMovement|IsMovingonGround (Variables|Character|GetCharacterMovement))
          (Audio|Components|Audio|Play _walk 0.0)))))
  (:Completed
    (Variables|Movement|SetisWalk false)
    (Variables|/Script/Engine.AudioComponent|SetVolumeMultiplier _walk 0.0)))

(event Input|EnhancedActionEvents|EnhancedInputActionSprint
  (params (ActionValue :type Boolean) (ElapsedSeconds :type Float%20%28double-precision%29) (TriggeredSeconds :type Float%20%28double-precision%29) (InputAction :type Input%20Action%20Object%20Reference :default "/Game/Inputs/Movement/Sprint.Sprint"))
  (bind _charactermovement (Variables|Character|GetCharacterMovement))
  (bind _walk (Variables|Default|Getwalk))
  ;[1 1 1] Character
  ;;[1 1 1] Sprint
  (:Started
    (if (Variables|Movement|GetcanRun)
      (Variables|/Script/Engine.CharacterMovementComponent|SetMaxWalkSpeed _charactermovement (Variables|Movement|GetMaxSpeedRun))
      (Variables|is|SetisShift true)
      (Audio|Components|Audio|SetSound _walk "/Game/SFX/Cue_Walk.Cue_Walk")))
  (:Completed
    (Variables|/Script/Engine.CharacterMovementComponent|SetMaxWalkSpeed _charactermovement (Variables|Movement|GetMaxSpeedWalk))
    (Variables|is|SetisShift false)
    (Audio|Components|Audio|SetSound _walk "/Game/SFX/Player/Cue_Walk_Better.Cue_Walk_Better")))

(event EventTick
  (params (DeltaSeconds :type Float%20%28single-precision%29))
  (if (Variables|Is|GetisPossessed)
    (Variables|Default|SetDelta%20Seconds DeltaSeconds)
    (Utilities|FlowControl|Sequence
      (:then_0
        (CallFunction|Outline)
        (CallFunction|Bobbing))
      (:then_1
        (CallFunction|SoundWalk)))))

(event EventBeginPlay
  ;[1 1 1] Character
  ;;[1 1 1] Initial
  (Utilities|FlowControl|Sequence
    (:then_0
      (bind _asplayer_controller (Utilities|Casting|CastToPlayerController (Pawn|GetController)))
      (Utilities|IsValid (PlayerController|LocalPlayerSubsystems|GetEnhancedInputLocalPlayerSubsystem _asplayer_controller)
        (:Is%20Valid
          (Input|AddMappingContext (PlayerController|LocalPlayerSubsystems|GetEnhancedInputLocalPlayerSubsystem _asplayer_controller) "/Game/Inputs/BasicInput.BasicInput" 0 "(bIgnoreAllPressedKeysUntilRelease=True,bForceImmediately=False,bNotifyUserSettings=False)"))))
    (:then_1
      (CallFunction|Begining)
      (CallFunction|Widgets))))

(fn ConstructionScript)

(fn Highlight
  (params (Object :type Actor%20Object%20Reference) (isOn :type Boolean) (Component :type Primitive%20Component%20Object%20Reference))
  (bind _robotwidget (Variables|Default|GetRobotWidget))
  (bind _hand_grab (Variables|/Game/UI/Game/Robot/WB_Robot.WB_Robot_C|GetHand_Grab _robotwidget))
  (Rendering|SetRenderCustomDepth (Variables|Default|GetLastHitComponent) isOn)
  (if isOn
    (Widget|SetVisibility _hand_grab "Visible")
    (switch name (Utilities|Array|Get(acopy) (Variables|/Script/Engine.Actor|GetTags (Variables|Default|GetLast%20Hit%20Actor)) 1)
      (:Default
        (Variables|Default|SetisGotValue false :!label _label)
        (Default|HidePrice (Variables|Default|GetRobotWidget))
        (return))
      (:gold
        (if (not (Variables|Default|GetisGotValue))
          (Variables|Default|SetisGotValue true)
          (bind _asbp_test_val_robot (Utilities|Casting|CastToBP_TestValRobot (Variables|Default|GetLast%20Hit%20Actor)))
          (Default|ShowPrice (Variables|Default|GetRobotWidget) (Variables|/Game/Blueprints/Robot/BP_TestValRobot.BP_TestValRobot_C|Getprice _asbp_test_val_robot))
          (return))))
    (else
      (Widget|SetVisibility _hand_grab "Hidden")
      (Variables|Default|SetLast%20Hit%20Actor 0)
      (Variables|Default|SetLastHitComponent 0)
      (goto _label))))

(fn DetermineValue
  (params (Target :type BP%20Test%20Val%20Robot%20Object%20Reference))
  (bind _price (Variables|/Game/Blueprints/Robot/BP_TestValRobot.BP_TestValRobot_C|Getprice Target))
  (Variables|Inventory|SetCurrentItemPrice _price)
  (if (Math|Integer|InRange(Integer) _price 100 1000) ; Inv = +1
    (bind _issuccess (CallFunction|AddItemtoInventory 1))
    (if (Math|Boolean|ORBoolean _issuccess (stale _issuccess_2) (stale _issuccess_3)) :!label _label
      (bind _output_get (Variables|Inventory|SetInventoryPrice (+ (Variables|Inventory|GetInventoryPrice) (Variables|Inventory|GetCurrentItemPrice))))
      (Development|PrintString (Utilities|String|ToString(Integer) _output_get)))
    (elif (Math|Integer|InRange(Integer) _price 1001 2000) ; Inv = +2
      (bind _issuccess_2 (CallFunction|AddItemtoInventory 2))
      (goto _label)
      (elif (Math|Integer|InRange(Integer) _price 2001 5000) ; Inv = +3
        (bind _issuccess_3 (CallFunction|AddItemtoInventory 3))
        (goto _label)
        (else
          (Development|PrintString (Utilities|String|Append "Current item price is: $" (Utilities|String|ToString(Integer) (Variables|Inventory|GetInventoryPrice))) true true "(R=1.000000,G=0.000000,B=0.000000,A=1.000000)")
          (Development|PrintString "Item price must be \"100 < item < 5000\"" true true "(R=1.000000,G=0.000000,B=0.000000,A=1.000000)"))))))

(fn AddItemtoInventory
  (params (Item%20Weight :type Integer))
  (bind _maxinventory (Variables|Inventory|GetMaxInventory))
  (if (< (Variables|Inventory|GetCurrentInventory) (Variables|Inventory|GetMaxInventory))
    (LocalVariables|SetisSuccsessfull true)
    (Variables|Inventory|SetCurrentInventory (+ (Variables|Inventory|GetCurrentInventory) Item%20Weight))
    (if (== (Variables|Inventory|GetCurrentInventory) _maxinventory)
      (Variables|Is|SetisOverflow false)
      (Variables|Movement|SetMaxSpeedWalk 3e+02)
      (Variables|Movement|SetcanRun true)
      (elif (< (Variables|Inventory|GetCurrentInventory) _maxinventory)
        (Variables|Is|SetisOverflow false)
        (Variables|Movement|SetMaxSpeedWalk 4e+02)
        (Variables|Movement|SetcanRun true)
        (else
          (Variables|Is|SetisOverflow true)
          (Variables|Movement|SetMaxSpeedWalk 2.5e+02)
          (Variables|Movement|SetcanRun false)
          (CallFunction|StopSprint))))
    (Default|CallOnUpdateVisualInv (Variables|Inventory|GetCurrentInventory))
    (Variables|/Script/Engine.CharacterMovementComponent|SetMaxWalkSpeed (Variables|Character|GetCharacterMovement) (Variables|Movement|GetMaxSpeedWalk))
    (return (LocalVariables|GetisSuccsessfull))
    (else
      (LocalVariables|SetisSuccsessfull false))))

(fn RemoveItemsfromInv
  (Variables|Inventory|SetInventoryPrice 0)
  (Variables|Inventory|SetCurrentInventory 0)
  (Variables|Is|SetisOverflow false)
  (Variables|Movement|SetcanRun true)
  (bind _output_get (Variables|Movement|SetMaxSpeedWalk 4e+02))
  (Variables|/Script/Engine.CharacterMovementComponent|SetMaxWalkSpeed (Variables|Character|GetCharacterMovement) _output_get)
  (Default|CallOnUpdateVisualInv))