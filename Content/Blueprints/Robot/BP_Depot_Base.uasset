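; BP_Depot_Base is a robot depot that spawns a separate basket actor and moves it during an extraction animation.
; On BeginPlay it stores the Scene component's transform and spawns BP_Depot_Basket there.
; ExtractLaunch plays the Extraction sequence, and while it runs, Tick copies the Scene component's transform onto the basket.
; A Sequencer event stops the following and resets the basket to its stored start transform.
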(event Custom|ExtractLaunch
  (Variables|Default|SetisAnim true)
  (Class|ActorSequenceComponent|PlaySequence (Variables|Default|Get%20Extraction)))

(event EventBeginPlay
  (bind _scene (Variables|Default|GetScene))
  (bind _returnvalue (Transformation|GetWorldTransform _scene))
  (Variables|Default|SetBaseBasketStartPos _returnvalue)
  (bind _returnvalue_2 (Game|SpawnActorfromClass "/Game/Blueprints/Robot/BP_Depot_Basket.BP_Depot_Basket_C" _returnvalue "Undefined" "MultiplyWithRoot" 0 0))
  (Variables|Default|SetBasket _returnvalue_2))

(event EventTick
  (params (DeltaSeconds :type Float%20%28single-precision%29))
  (if (Variables|Default|GetisAnim)
    (Transformation|SetActorTransform (Variables|Default|GetBasket) (Transformation|GetWorldTransform (Variables|Default|GetScene)))))

(event Custom|SequenceEvent
  (Variables|Default|SetisAnim false)
  (Transformation|SetActorTransform (Variables|Default|GetBasket) (Variables|Default|GetBaseBasketStartPos)))

(fn ConstructionScript)