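; BP_AFESystem is a resource manager actor that drains robot Energy and a Fuel pool during play.
; It finds the robot, turret and attack node on BeginPlay, then polls their flags each Tick through three macros.
; Possessed-robot energy drains by movement and flashlight state, broadcasting updates, while turret shots and occupied attack nodes consume Fuel.
; Robot death is an empty event, and fuel depletion only prints debug text.
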(event Custom|RobotDies
  ;[0.15 0.15 0.15 0.5] Robot run out of fuel
)

(event EventBeginPlay
  (Utilities|FlowControl|Sequence
    (:then_0
      (bind _returnvalue (Actor|GetActorOfClass "/Game/Blueprints/Robot/BP_Robot.BP_Robot_C"))
      (Variables|Energy|SetRobotRef _returnvalue))
    (:then_1
      (bind _returnvalue_2 (Actor|GetActorOfClass "/Game/Blueprints/Enemy/BP_Turret.BP_Turret_C"))
      (Variables|Fuel|SetTurretRef _returnvalue_2))
    (:then_2
      (bind _returnvalue_3 (Actor|GetActorOfClass "/Game/Blueprints/Enemy/BP_AttackNode.BP_AttackNode_C"))
      (Variables|Fuel|SetEnemyAttack _returnvalue_3))))

(event Collision|EventActorBeginOverlap
  (params (OtherActor :type Actor%20Object%20Reference)))

(event EventTick
  (params (DeltaSeconds :type Float%20%28single-precision%29))
  (Variables|Default|SetDelta%20Seconds DeltaSeconds)
  (Utilities|FlowControl|Sequence
    (:then_0
      (if (Variables|/Game/Blueprints/Robot/BP_Robot.BP_Robot_C|GetisPossessed (Variables|Energy|GetRobotRef))
        (Utilities|EnergyM
          (:then
            (Default|CallOnEnergyUpdate (Variables|Energy|GetEnergy)))
          (:RobotDies
            (CallFunction|RobotDies)))))
    (:then_1
      (if (Variables|/Game/Blueprints/Enemy/BP_Turret.BP_Turret_C|GetShoot (Variables|Fuel|GetTurretRef))
        (Utilities|ShootM)))
    (:then_2
      (if (Variables|/Game/Blueprints/Enemy/BP_EnemyPoint.BP_EnemyPoint_C|GetOccupied (Variables|Fuel|GetEnemyAttack))
        (Utilities|EnemyAttackM)))))

(fn ConstructionScript)